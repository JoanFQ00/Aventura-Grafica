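; Interactable trigger actor that opens a card-target minigame to activate a door.
; On BeginPlay it creates the minigame, CardTarget and interact-prompt widgets and binds to CardTarget's DoorOpened event.
; Overlap animates the prompt in and out; pressing IA_Interaction inside shows the minigame with mouse input.
; Once DoorOpened fires, the prompt switches to exit text and interacting removes all widgets and restores game-only input.
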(event `self.ReceiveBeginPlay`
  (bind _returnvalue (`|CreateWidget` "/Game/MenusAndUI/Minigame/BP_Minigame.BP_Minigame_C"))
  (set `self.Ref_MiniGame` _returnvalue)
  (bind _returnvalue_2 (`|CreateWidget` "/Game/MenusAndUI/Minigame/CardTarget.CardTarget_C"))
  (set `self.Ref_CardTargMG` _returnvalue_2)
  (bind _returnvalue_3 (`|CreateWidget` "/Game/MenusAndUI/WG_Interact.WG_Interact_C"))
  (set `self.Ref_InteractWG` _returnvalue_3)
  (`self.EnableInput` (`GameplayStatics.GetPlayerController` 0))
  (add `/Game/MenusAndUI/Minigame/CardTarget.DoorOpened` (`self.Ref_CardTargMG`) (delegate `CustomEvent`)))

(event `self.ReceiveActorBeginOverlap`
  (params (OtherActor :type "Actor Object Reference"))
  (bind _ref_interactwg (`self.Ref_InteractWG`))
  (`UserWidget.AddToViewport` (`self.Ref_InteractWG`) 0)
  (`UserWidget.PlayAnimation` _ref_interactwg (`/Game/MenusAndUI/WG_Interact.EnterInteract` _ref_interactwg) 0.0 1 "Forward" 1.0 false)
  (set `self.charcterInside` true))

(event `CustomEvent`
  (set `self.DoorActivated` true)
  (`Widget.SetVisibility` (`/Game/MenusAndUI/WG_Interact.Interacttext` (`self.Ref_InteractWG`)) "Hidden")
  (`Widget.SetVisibility` (`/Game/MenusAndUI/WG_Interact.Exittext` (`self.Ref_InteractWG`)) "Visible"))

(event `self.ReceiveActorEndOverlap`
  (params (OtherActor :type "Actor Object Reference"))
  (bind _ref_interactwg (`self.Ref_InteractWG`))
  (`UserWidget.PlayAnimationReverse` _ref_interactwg (`/Game/MenusAndUI/WG_Interact.EnterInteract` _ref_interactwg) 1.0 false)
  (`KismetSystemLibrary.Delay` 0.75)
  (set `self.charcterInside` false)
  (`Widget.RemoveFromParent` (`self.Ref_MiniGame`))
  (`Widget.RemoveFromParent` (`self.Ref_CardTargMG`))
  (`Widget.RemoveFromParent` (`self.Ref_InteractWG`)))

(event `EnhancedInput|/Game/Interactables/IA_Interaction`
  (params (ActionValue :type Boolean) (ElapsedSeconds :type "Float (double-precision)") (TriggeredSeconds :type "Float (double-precision)") (InputAction :type "InputAction Object Reference" :default "/Game/Interactables/IA_Interaction.IA_Interaction"))
  (bind _returnvalue (`GameplayStatics.GetPlayerController` 0))
  (bind _returnvalue_2 (`GameplayStatics.GetPlayerController` 0))
  (:`Started`
    (if (`self.charcterInside`)
      (`Widget.SetVisibility` (`/Game/MenusAndUI/WG_Interact.Interacttext` (`self.Ref_InteractWG`)) "Visible")
      (if (`self.DoorActivated`)
        (`WidgetLayoutLibrary.RemoveAllWidgets`)
        (`WidgetBlueprintLibrary.SetInputMode_GameOnly` _returnvalue_2)
        (set `PlayerController.bShowMouseCursor` false _returnvalue_2)
        (else
          (`UserWidget.AddToViewport` (`self.Ref_MiniGame`) 0)
          (`UserWidget.AddToViewport` (`self.Ref_CardTargMG`) 0)
          (`WidgetBlueprintLibrary.SetInputMode_GameAndUIEx` _returnvalue null)
          (set `PlayerController.bShowMouseCursor` true _returnvalue)
          (`Widget.SetVisibility` (`/Game/MenusAndUI/WG_Interact.Exittext` (`self.Ref_InteractWG`)) "Hidden")
          (`Widget.SetVisibility` (`/Game/MenusAndUI/WG_Interact.Interacttext` (`self.Ref_InteractWG`)) "Visible"))))))

(fn `UserConstructionScript`)